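; BP_Elias is the player character, adding Enhanced Input for movement, jump and interaction, plus a bodycam overlay with a blink animation.
; Look input aims FlashlightSpot within a clamped deadzone, turning the controller only in yaw once the horizontal limit is reached.
; Pressing interact runs a short debug-drawn trace along the flashlight, sends BPI_Interaction focus messages, then triggers interaction on a valid target.
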(event Input|EnhancedActionEvents|EnhancedInputActionIA_Interact
  (params (ActionValue :type Boolean) (ElapsedSeconds :type Float%20%28double-precision%29) (TriggeredSeconds :type Float%20%28double-precision%29) (InputAction :type Input%20Action%20Object%20Reference :default "/Game/_Game/Input/Actions/IA_Interact.IA_Interact"))
  (bind _currentinteractable (Variables|Default|GetCurrentInteractable))
  (:Started
    (CallFunction|PerformInteractionTrace)
    (Utilities|IsValid _currentinteractable
      (:Is%20Valid
        (Class|BPIInteraction|OnInteract(Message) _currentinteractable)))))

(event EventBeginPlay
  (bind _asplayer_controller (Utilities|Casting|CastToPlayerController (Pawn|GetController)))
  (Input|AddMappingContext (PlayerController|LocalPlayerSubsystems|GetEnhancedInputLocalPlayerSubsystem _asplayer_controller) "/Game/_Game/Input/IMC_Default.IMC_Default" 0 "(bIgnoreAllPressedKeysUntilRelease=True,bForceImmediately=False,bNotifyUserSettings=False)")
  (bind _returnvalue (UserInterface|CreateWidget "/Game/_Game/UI/WBP_BodycamOverlay.WBP_BodycamOverlay_C"))
  (UserInterface|Viewport|AddtoViewport _returnvalue 0)
  (UserInterface|Animation|PlayAnimation _returnvalue (Variables|/Game/_Game/UI/WBP_BodycamOverlay.WBP_BodycamOverlay_C|GetBlinkAnim _returnvalue) 0.0 0 "Forward" 1.0 false))

(event Collision|EventActorBeginOverlap
  (params (OtherActor :type Actor%20Object%20Reference)))

(event EventTick
  (params (DeltaSeconds :type Float%20%28single-precision%29)))

(event Input|EnhancedActionEvents|EnhancedInputActionIA_Move
  (params (ActionValue :type Vector%202D%20Structure) (ElapsedSeconds :type Float%20%28double-precision%29) (TriggeredSeconds :type Float%20%28double-precision%29) (InputAction :type Input%20Action%20Object%20Reference :default "/Game/_Game/Input/Actions/IA_Move.IA_Move"))
  (CallFunction|Move (.x ActionValue) (.y ActionValue)))

(event Input|EnhancedActionEvents|EnhancedInputActionIA_Look
  (params (ActionValue :type Vector%202D%20Structure) (ElapsedSeconds :type Float%20%28double-precision%29) (TriggeredSeconds :type Float%20%28double-precision%29) (InputAction :type Input%20Action%20Object%20Reference :default "/Game/_Game/Input/Actions/IA_Look.IA_Look"))
  (CallFunction|Aim (.x ActionValue) (.y ActionValue)))

(event Input|EnhancedActionEvents|EnhancedInputActionIA_Jump
  (params (ActionValue :type Boolean) (ElapsedSeconds :type Float%20%28double-precision%29) (TriggeredSeconds :type Float%20%28double-precision%29) (InputAction :type Input%20Action%20Object%20Reference :default "/Game/_Game/Input/Actions/IA_Jump.IA_Jump"))
  (Utilities|FlowControl|FlipFlop
    (:A
      (Character|Jump))
    (:B
      (Character|StopJumping))))

(fn ConstructionScript)

(fn Move
  (params (Left%20/%20Right :type Float%20%28double-precision%29) (Forward%20/%20Back :type Float%20%28double-precision%29))
  (Pawn|Input|AddMovementInput (Transformation|GetActorRightVector) Left%20/%20Right false)
  (Pawn|Input|AddMovementInput (Transformation|GetActorForwardVector) Forward%20/%20Back false))

(fn Aim
  (params (Yaw :type Float%20%28double-precision%29) (Pitch :type Float%20%28double-precision%29))
  (bind _deadzonelimit_y (Variables|Default|GetDeadzoneLimit_Y))
  (bind _deadzonelimit_x (Variables|Default|GetDeadzoneLimit_X))
  (bind _returnvalue (* _deadzonelimit_x -1.0))
  (Variables|Default|SetFlashlightPitch (Math|Float|Clamp(Float) (+ (Variables|Default|GetFlashlightPitch) (* Pitch -1.0)) (* _deadzonelimit_y -1.0) _deadzonelimit_y))
  (Variables|Default|SetFlashlightYaw (Math|Float|Clamp(Float) (+ (Variables|Default|GetFlashlightYaw) (* Yaw 1.0)) _returnvalue _deadzonelimit_x))
  (if (or (>= (Variables|Default|GetFlashlightYaw) _deadzonelimit_x) (<= (Variables|Default|GetFlashlightYaw) _returnvalue))
    (Pawn|Input|AddControllerYawInput Yaw))
  (Transformation|SetRelativeRotation (Variables|Default|GetFlashlightSpot) (Math|Rotator|MakeRotator 0.0 (Variables|Default|GetFlashlightPitch) (Variables|Default|GetFlashlightYaw)) false false))

(fn PerformInteractionTrace
  (bind _flashlightspot (Variables|Default|GetFlashlightSpot))
  (bind _returnvalue (Transformation|GetWorldLocation _flashlightspot))
  (bind _outhit (Collision|LineTraceByChannel _returnvalue (+ _returnvalue (* (Math|Vector|GetForwardVector _flashlightspot) 3e+02)) "TraceTypeQuery1" false 0 "ForDuration"))
  (if (Utilities|DoesObjectImplementInterface (.HitActor (Collision|BreakHitResult _outhit)) "/Game/_Game/Blueprints/Core/Interfaces/BPI_Interaction.BPI_Interaction_C")
    (bind _output_get (Variables|Default|SetCurrentInteractable (.HitActor (Collision|BreakHitResult _outhit))))
    (Class|BPIInteraction|OnFocus(Message) _output_get)
    (else
      (Class|BPIInteraction|OnLostFocus(Message) (.HitActor (Collision|BreakHitResult _outhit)))
      (Variables|Default|SetCurrentInteractable 0))))