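; BP_Detective is a player character with Enhanced Input movement, mouse-style look and hitscan shooting.
; BeginPlay adds the detective mapping context, and the move and look actions drive the Move and Aim functions, with pitch inverted.
; Firing spends ammo and runs a short, debug-drawn Visibility line trace forward from EyeCam, applying damage to any hit actor.
; A DoOnce gates each shot and resets after the trace, hit or miss.
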(event Input|EnhancedActionEvents|EnhancedInputActionIA_Fire
  (params (ActionValue :type Boolean) (ElapsedSeconds :type Float%20%28double-precision%29) (TriggeredSeconds :type Float%20%28double-precision%29) (InputAction :type Input%20Action%20Object%20Reference :default "/Game/_Game/Input/Actions/IA_Fire.IA_Fire"))
  (bind _eyecam (Variables|Default|GetEyeCam))
  (bind _returnvalue (Transformation|GetWorldLocation _eyecam))
  (:Started
    (if (> (Variables|Default|GetCurrentAmmo) 0)
      (Utilities|FlowControl|DoOnce false :!label _label
        (:Completed
          (Variables|Default|SetCurrentAmmo (- (Variables|Default|GetCurrentAmmo) 1))
          (bind (_outhit _returnvalue_2) (Collision|LineTraceByChannel _returnvalue (+ _returnvalue (* (Math|Vector|GetForwardVector _eyecam) 5e+02)) "TraceTypeQuery1" false 0 "ForDuration"))
          (if _returnvalue_2
            (Game|Damage|ApplyDamage (.HitActor (Collision|BreakHitResult _outhit)) 5e+01 (Pawn|GetController) self "/Script/Engine.DamageType")
            (goto _label Reset)
            (else
              (goto _label Reset))))))))

(event EventBeginPlay
  (bind _asplayer_controller (Utilities|Casting|CastToPlayerController (Pawn|GetController)))
  (Input|AddMappingContext (PlayerController|LocalPlayerSubsystems|GetEnhancedInputLocalPlayerSubsystem _asplayer_controller) "/Game/_Game/Input/IMC_Detective.IMC_Detective" 0 "(bIgnoreAllPressedKeysUntilRelease=True,bForceImmediately=False,bNotifyUserSettings=False)"))

(event Collision|EventActorBeginOverlap
  (params (OtherActor :type Actor%20Object%20Reference)))

(event EventTick
  (params (DeltaSeconds :type Float%20%28single-precision%29)))

(event Input|EnhancedActionEvents|EnhancedInputActionIA_Move
  (params (ActionValue :type Vector%202D%20Structure) (ElapsedSeconds :type Float%20%28double-precision%29) (TriggeredSeconds :type Float%20%28double-precision%29) (InputAction :type Input%20Action%20Object%20Reference :default "/Game/_Game/Input/Actions/IA_Move.IA_Move"))
  (CallFunction|Move (.x ActionValue) (.y ActionValue)))

(event Input|EnhancedActionEvents|EnhancedInputActionIA_Look
  (params (ActionValue :type Vector%202D%20Structure) (ElapsedSeconds :type Float%20%28double-precision%29) (TriggeredSeconds :type Float%20%28double-precision%29) (InputAction :type Input%20Action%20Object%20Reference :default "/Game/_Game/Input/Actions/IA_Look.IA_Look"))
  (CallFunction|Aim (.x ActionValue) (.y ActionValue)))

(fn ConstructionScript)

(fn Move
  (params (Left%20/%20Right :type Float%20%28double-precision%29) (Forward%20/%20Back :type Float%20%28double-precision%29))
  (Pawn|Input|AddMovementInput (Transformation|GetActorRightVector) Left%20/%20Right false)
  (Pawn|Input|AddMovementInput (Transformation|GetActorForwardVector) Forward%20/%20Back false))

(fn Aim
  (params (Yaw :type Float%20%28double-precision%29) (Pitch :type Float%20%28double-precision%29))
  (Pawn|Input|AddControllerYawInput Yaw)
  (Pawn|Input|AddControllerPitchInput (* Pitch -1.0)))