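; BP_Director is the player-controlled Director character, with a toggleable Divine Mode for using powers on entities.
; Enhanced Input drives look and movement, with the jump input switching to Flying while held.
; Toggling Divine Mode creates or removes the HUD and fades eye overlay materials through a timeline.
; Ability inputs select Smite or Telekinesis; attack implements only Smite, a camera line trace dealing lethal-scale damage to BP_Entity.
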(event Input|EnhancedActionEvents|EnhancedInputActionIA_Move
  (params (ActionValue :type Vector%202D%20Structure) (ElapsedSeconds :type Float%20%28double-precision%29) (TriggeredSeconds :type Float%20%28double-precision%29) (InputAction :type Input%20Action%20Object%20Reference :default "/Game/_Game/Input/Actions/IA_Move.IA_Move"))
  (bind _returnvalue (Pawn|GetControlRotation :!class /Script/Engine.Pawn))
  (Pawn|Input|AddMovementInput (Math|Vector|GetRightVector (Math|Rotator|MakeRotator (.roll _returnvalue) 0.0 (.yaw _returnvalue))) (.x ActionValue) false)
  (Pawn|Input|AddMovementInput (Math|Vector|GetForwardVector (Math|Rotator|MakeRotator 0.0 0.0 (.yaw (Pawn|GetControlRotation :!class /Script/Engine.Pawn)))) (.y ActionValue) false))

(event Input|EnhancedActionEvents|EnhancedInputActionIA_Look
  (params (ActionValue :type Vector%202D%20Structure) (ElapsedSeconds :type Float%20%28double-precision%29) (TriggeredSeconds :type Float%20%28double-precision%29) (InputAction :type Input%20Action%20Object%20Reference :default "/Game/_Game/Input/Actions/IA_Look.IA_Look"))
  (Pawn|Input|AddControllerYawInput (.x ActionValue))
  (Pawn|Input|AddControllerPitchInput (.y ActionValue)))

(event Input|EnhancedActionEvents|EnhancedInputActionIA_Jump
  (params (ActionValue :type Boolean) (ElapsedSeconds :type Float%20%28double-precision%29) (TriggeredSeconds :type Float%20%28double-precision%29) (InputAction :type Input%20Action%20Object%20Reference :default "/Game/_Game/Input/Actions/IA_Jump.IA_Jump"))
  (bind _charactermovement (Variables|Character|GetCharacterMovement))
  (:Triggered
    (Pawn|Input|AddMovementInput "0.000000,0.000000,0.000000" 1.0 false))
  (:Started
    (Pawn|Components|CharacterMovement|SetMovementMode _charactermovement "MOVE_Flying" 0))
  (:Completed
    (Pawn|Components|CharacterMovement|SetMovementMode _charactermovement "MOVE_Walking" 0)))

(event Input|EnhancedActionEvents|EnhancedInputActionIA_ToggleMode
  (params (ActionValue :type Boolean) (ElapsedSeconds :type Float%20%28double-precision%29) (TriggeredSeconds :type Float%20%28double-precision%29) (InputAction :type Input%20Action%20Object%20Reference :default "/Game/_Game/Input/Actions/IA_ToggleMode.IA_ToggleMode"))
  (:Started
    (Utilities|FlowControl|FlipFlop
      (:A
        (Variables|Default|SetIsDivineMode true)
        (Utilities|FlowControl|Sequence
          (:then_0
            (bind _returnvalue (UserInterface|CreateWidget "/Game/_Game/UI/WBP_DirectorHUD.WBP_DirectorHUD_C"))
            (Variables|Default|SetHUD_Ref _returnvalue)
            (UserInterface|Viewport|AddtoViewport _returnvalue 0)
            (Default|UpdateActiveIcon (Variables|Default|GetHUD_Ref) 1))
          (:then_1
            (bind _opacity (Timeline|Timeline Play)
              (:Update
                (Rendering|Material|SetScalarParameterValue (Variables|Default|GetMat_Eye_L) "OpacityAmount" _opacity :!class /Script/Engine.MaterialInstanceDynamic)
                (Rendering|Material|SetScalarParameterValue (Variables|Default|GetMat_Eye_R) "OpacityAmount" _opacity :!class /Script/Engine.MaterialInstanceDynamic))))))
      (:B
        (Variables|Default|SetIsDivineMode false)
        (Utilities|FlowControl|Sequence
          (:then_0
            (Timeline|Timeline Reverse))
          (:then_1
            (Widget|RemovefromParent (Variables|Default|GetHUD_Ref))
            (Variables|Default|SetHUD_Ref 0)))))))

(event Input|EnhancedActionEvents|EnhancedInputActionIA_Ability_1
  (params (ActionValue :type Boolean) (ElapsedSeconds :type Float%20%28double-precision%29) (TriggeredSeconds :type Float%20%28double-precision%29) (InputAction :type Input%20Action%20Object%20Reference :default "/Game/_Game/Input/Actions/IA_Ability_1.IA_Ability_1"))
  (:Started
    (Variables|Default|SetSelectedPowerIndex 1)
    (Default|UpdateActiveIcon (Variables|Default|GetHUD_Ref) 1)
    (Development|PrintString "Poder: SMITE")))

(event Input|EnhancedActionEvents|EnhancedInputActionIA_Ability_2
  (params (ActionValue :type Boolean) (ElapsedSeconds :type Float%20%28double-precision%29) (TriggeredSeconds :type Float%20%28double-precision%29) (InputAction :type Input%20Action%20Object%20Reference :default "/Game/_Game/Input/Actions/IA_Ability_2.IA_Ability_2"))
  (:Started
    (Variables|Default|SetSelectedPowerIndex 2)
    (Default|UpdateActiveIcon (Variables|Default|GetHUD_Ref) 2)
    (Development|PrintString "Poder: TELEKINESIS")))

(event Input|EnhancedActionEvents|EnhancedInputActionIA_Attack
  (params (ActionValue :type Boolean) (ElapsedSeconds :type Float%20%28double-precision%29) (TriggeredSeconds :type Float%20%28double-precision%29) (InputAction :type Input%20Action%20Object%20Reference :default "/Game/_Game/Input/Actions/IA_Attack.IA_Attack"))
  (bind _camera (Variables|Default|GetCamera))
  (bind _returnvalue (Transformation|GetWorldLocation _camera))
  (:Started
    (if (Variables|Default|GetIsDivineMode)
      (switch int (Variables|Default|GetSelectedPowerIndex)
        (:1
          (bind (_outhit _returnvalue_2) (Collision|LineTraceByChannel _returnvalue (+ _returnvalue (* (Math|Vector|GetForwardVector _camera) 2e+03)) "TraceTypeQuery1" false 0 "ForDuration"))
          (if _returnvalue_2
            (bind _asbp_entity (Utilities|Casting|CastToBP_Entity (.HitActor (Collision|BreakHitResult _outhit))))
            (Game|Damage|ApplyDamage _asbp_entity 9999.0 (Pawn|GetController) self "/Script/Engine.DamageType")))))))

(event EventBeginPlay
  (bind _asplayer_controller (Utilities|Casting|CastToPlayerController (Pawn|GetController)))
  (Input|AddMappingContext (PlayerController|LocalPlayerSubsystems|GetEnhancedInputLocalPlayerSubsystem _asplayer_controller) "/Game/_Game/Input/IMC_Diretor.IMC_Diretor" 0 "(bIgnoreAllPressedKeysUntilRelease=True,bForceImmediately=False,bNotifyUserSettings=False)")
  (bind _returnvalue (Rendering|Material|CreateDynamicMaterialInstance (Variables|Default|GetLeftEye_Overlay) 0 "/Game/_Game/Assets/Materials/M_Eye_Overlay.M_Eye_Overlay" "None" :!class /Script/Engine.PrimitiveComponent))
  (Variables|Default|SetMat_Eye_L _returnvalue)
  (bind _returnvalue_2 (Rendering|Material|CreateDynamicMaterialInstance (Variables|Default|GetRightEye_Overlay) 0 "/Game/_Game/Assets/Materials/M_Eye_Overlay.M_Eye_Overlay" "None" :!class /Script/Engine.PrimitiveComponent))
  (Variables|Default|SetMat_Eye_R _returnvalue_2))

(fn ConstructionScript)