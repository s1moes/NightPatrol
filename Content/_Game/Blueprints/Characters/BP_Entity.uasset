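; BP_Entity is a character Blueprint that gives an entity health, damage handling and a ragdoll death.
; AnyDamage subtracts from Health while the entity is alive, prints an "enemy hit" message in Portuguese and calls Die when health runs out.
; Die sets IsDead to block further damage, stops movement, detaches the controller and switches the mesh to simulated ragdoll physics.
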(event Custom|Die
  (Variables|Default|SetIsDead true)
  (Components|Movement|StopMovementImmediately (Variables|Character|GetCharacterMovement))
  (Class|Pawn|DetachfromControllerPendingDestroy)
  (Collision|SetCollisionProfileName (Variables|Character|GetMesh) "Ragdoll" true :!class /Script/Engine.PrimitiveComponent)
  (Physics|SetSimulatePhysics (Variables|Character|GetMesh) true))

(event EventBeginPlay)

(event Collision|EventActorBeginOverlap
  (params (OtherActor :type Actor%20Object%20Reference)))

(event EventTick
  (params (DeltaSeconds :type Float%20%28single-precision%29)))

(event Game|Damage|EventAnyDamage
  (params (Damage :type Float%20%28single-precision%29) (DamageType :type Damage%20Type%20Object%20Reference) (InstigatedBy :type Controller%20Object%20Reference) (DamageCauser :type Actor%20Object%20Reference))
  (if (not (Variables|Default|GetIsDead))
    (Variables|Default|SetHealth (- (Variables|Default|GetHealth) Damage))
    (Development|PrintString "Inimigo atingido!")
    (if (<= (Variables|Default|GetHealth) 0.0)
      (CallFunction|Die))))

(fn ConstructionScript)