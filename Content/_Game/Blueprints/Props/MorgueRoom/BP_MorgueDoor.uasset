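; BP_MorgueDoor is the interactable morgue door, which can require a key held by the player character, BP_Elias.
; On interact, a timeline swings DoorPanel open in yaw if no key is required or Elias has the morgue key.
; Without the key, a DoOnce sets a Portuguese objective to find it in the security room and unhides the BP_Keycard found through GetActorOfClass.
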(event EventBeginPlay)

(event Collision|EventActorBeginOverlap
  (params (OtherActor :type Actor%20Object%20Reference)))

(event EventTick
  (params (DeltaSeconds :type Float%20%28single-precision%29)))

(event EventOnInteract
  (bind _asbp_elias (Utilities|Casting|CastToBP_Elias (Game|Player|GetPlayerPawn 0)))
  (if (Variables|Default|GetRequiresKey)
    (if (Variables|/Game/_Game/Blueprints/Characters/BP_Elias.BP_Elias_C|GetHasKeyMorgue _asbp_elias)
      (bind _newtrack_0 (Timeline|OpenDoorTL Play)
        (:Update
          (Transformation|SetRelativeRotation (Variables|Default|GetDoorPanel) (Math|Rotator|MakeRotator 0.0 0.0 _newtrack_0) false false)))
      (else
        (Utilities|FlowControl|DoOnce false
          (:Completed
            (bind _asbp_elias_2 (Utilities|Casting|CastToBP_Elias (Game|Player|GetPlayerPawn 0)))
            (Default|UpdateObjective _asbp_elias_2 "ENCONTRAR CHAVE NA SALA DE SEGURANÇA!")
            (bind _returnvalue (Actor|GetActorOfClass "/Game/_Game/Blueprints/Props/SecurityRoom/BP_Keycard.BP_Keycard_C"))
            (Rendering|SetActorHiddenInGame _returnvalue false)))))
    (else
      (Timeline|OpenDoorTL Play))))

(fn ConstructionScript)